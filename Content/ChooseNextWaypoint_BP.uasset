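; Behavior tree task that picks the next patrol waypoint for an AI-controlled ThirdPersonCharacter.
; It reads the Waypoints array from the controlled pawn, then writes the entry at the blackboard's NextWaypointIndex into the NextWaypoint key.
; It then increments the index with a modulo wrap, so the route loops, and finishes with success.
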(event EventReceiveExecuteAI
  (params (OwnerController :type AI%20Controller%20Object%20Reference) (ControlledPawn :type Pawn%20Object%20Reference))
  (CallFunction|GetWaypoints ControlledPawn)
  (bind _waypointindex (CallFunction|SetNextWaypoint))
  (CallFunction|CycletoNextWaypoint _waypointindex)
  (AI|BehaviorTree|FinishExecute true))

(fn GetWaypoints
  (params (Object :type Object%20Object%20Reference))
  (bind _asthird_person_character (Utilities|Casting|CastToThirdPersonCharacter Object))
  (Variables|Default|SetWay%20points (Variables|/Game/ThirdPersonCPP/Blueprints/ThirdPersonCharacter.ThirdPersonCharacter_C|GetWaypoints _asthird_person_character)))

(fn SetNextWaypoint
  (bind _nextwaypointindex (Variables|Default|GetNextWaypointIndex))
  (bind _returnvalue (Class|BTFunctionLibrary|GetBlackboardValueasInt _nextwaypointindex))
  (Class|BTFunctionLibrary|SetBlackboardValueasObject (Variables|Default|GetNextWaypoint) (Utilities|Array|Get(acopy) (Variables|Default|GetWay%20points) _returnvalue))
  (return _returnvalue))

(fn CycletoNextWaypoint
  (params (WaypointIndex :type Integer))
  (Class|BTFunctionLibrary|SetBlackboardValueasInt (Variables|Default|GetNextWaypointIndex) (Math|Integer|%(Integer) (+ WaypointIndex 1) (Utilities|Array|Length (Variables|Default|GetWay%20points)))))