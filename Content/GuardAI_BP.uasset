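; AI controller for a guard that runs a patrol behavior tree on its controlled pawn.
; On BeginPlay it sets up the PatrolLogic blackboard, seeds its Waypoint key, then starts the Patrol tree.
; The seed is the first entry in the ThirdPersonCharacter pawn's Waypoints array; if the cast fails, it only prints an error.
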(event EventBeginPlay
  (bind _blackboardcomponent (Class|AIController|UseBlackboard "/Game/PatrolLogic.PatrolLogic"))
  (CallFunction|SelectWaypoint _blackboardcomponent)
  (AI|RunBehaviorTree "/Game/Patrol.Patrol"))

(event EventTick
  (params (DeltaSeconds :type Float%20%28single-precision%29)))

(fn ConstructionScript)

(fn SelectWaypoint
  (params (BlackboardComponent :type Blackboard%20Component%20Object%20Reference))
  (bind _asthird_person_character (Utilities|Casting|CastToThirdPersonCharacter (Pawn|GetControlledPawn))
    (:then
      (AI|Components|Blackboard|SetValueasObject BlackboardComponent (Utilities|Name|MakeLiteralName "Waypoint") (Utilities|Array|Get(acopy) (Variables|/Game/ThirdPersonCPP/Blueprints/ThirdPersonCharacter.ThirdPersonCharacter_C|GetWaypoints _asthird_person_character))))
    (:CastFailed
      (Development|PrintString "No Third Person Character found"))))